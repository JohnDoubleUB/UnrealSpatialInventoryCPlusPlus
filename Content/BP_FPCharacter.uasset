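; First-person character Blueprint that owns the player's inventory screen.
; On BeginPlay it caches the player controller and creates an inventory widget bound to its inventory component.
; OnInventoryEnabled has no logic wired to it.
; A disconnected branch would add or remove the widget, switch input mode and toggle the mouse cursor, with Enabled true hiding the inventory.
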(event `self.ReceiveBeginPlay`
  ;[1 1 1] Done
  (set `self.PlayerController` (`self.Get Player Controller`))
  (bind _returnvalue (`|CreateWidget` "/Game/Inventory/SpatialInventory/BP_Inventory_Widget2.BP_Inventory_Widget2_C" null (`self.BP_InventoryComponent`) 50.0))
  (set `self.SI_InventoryWidget` _returnvalue))

(event `self.OnInventoryEnabled`
  (params (enabled :type Boolean))
  ;[1 1 1] Done
)

(fn `Get Player Controller`
  (returns (`AsPlayer Controller` :type "PlayerController Object Reference"))
  (return (cast `PlayerController` (`self.GetController` self) :!pure true)))

(fn `UserConstructionScript`)
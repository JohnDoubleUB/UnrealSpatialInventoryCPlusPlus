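; Spatial inventory component that stores pickups in a flat Columns-by-Rows array, with multi-tile items filling every slot they cover.
; TryAddItem scans for a top-left slot using IsRoomAvailable, then AddItemAtIndex writes the footprint and sets IsDirty.
; A shared footprint macro walks tiles through index/tile conversion.
; As wired, room checks receive the slot's occupant instead of the new item, and tile validation compares upper bounds to zero, so always fails.
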(event `self.ReceiveBeginPlay`
  (`KismetArrayLibrary.Array_Resize` (`self.InventoryGrid`) (* (`self.Columns`) (`self.Rows`))))

(fn `AddItemAtIndex`
  (params (PickupObject :type "/Game/Inventory/BP_UIPickup Object Reference") (TopLeftCorner :type Integer))
  (bind _tile (`self.ForEachPickupSpaceIndex` PickupObject TopLeftCorner)
    (:`LoopBody`
      (`KismetArrayLibrary.Array_Set` (`self.InventoryGrid`) (`self.TileToIndex` _tile) PickupObject))
    (:`Completed`
      (set `self.IsDirty` true))))

(fn `GetItemAtIndex`
  (params (Index :type Integer))
  (returns (Valid :type Boolean) (ItemObject :type "/Game/Inventory/BP_UIPickup Object Reference"))
  (if (`KismetArrayLibrary.Array_IsValidIndex` (`self.InventoryGrid`) Index)
    (return true (`|GetArrayItem` (`self.InventoryGrid`) Index))
    (else
      (return false null))))

(fn `IndexToTile`
  (params (Index :type Integer))
  (returns (Tile :type "/Game/Inventory/SpatialInventory/STile Structure"))
  (bind _columns (`self.Columns`))
  (return (make `/Game/Inventory/SpatialInventory/STile` (mod Index _columns) (/ Index _columns))))

(fn `IsRoomAvailable`
  (params (UIPickup :type "/Game/Inventory/BP_UIPickup Object Reference") (TopLeftIndex :type Integer))
  (returns (result :type Boolean))
  (`|ExecutionSequence`
    (:`then_0`
      (bind _tile (`self.ForEachPickupSpaceIndex` UIPickup TopLeftIndex)
        (:`LoopBody`
          (`self.isValidInventoryTile` _tile
            (:`true`
              (bind (_valid _itemobject) (`self.GetItemAtIndex` (`self.TileToIndex` _tile)))
              (if _valid
                (`/Engine/EditorBlueprintResources/StandardMacros.IsValid` _itemobject
                  (:`Is Valid`
                    (return false)))
                (else
                  (return false))))
            (:`false`
              (return false))))))
    (:`then_1`
      (return true))))

(fn `TileToIndex`
  (params (Tile :type "/Game/Inventory/SpatialInventory/STile Structure"))
  (returns (Index :type Integer))
  (bind (_x _y) (break `/Game/Inventory/SpatialInventory/STile` Tile))
  (return (+ _x (* _y (`self.Columns`)))))

(fn `TryAddItem`
  (params (ItemUIPickup :type "/Game/Inventory/BP_UIPickup Object Reference"))
  (returns (Success :type Boolean))
  (`/Engine/EditorBlueprintResources/StandardMacros.IsValid` ItemUIPickup
    (:`Is Valid`
      (for (_array_element _array_index) (`self.InventoryGrid`)
        (bind _result (`self.IsRoomAvailable` _array_element _array_index))
        (if _result
          (`self.AddItemAtIndex` ItemUIPickup _array_index)
          (return true)))
      (return false))
    (:`Is Not Valid`
      (return false))))
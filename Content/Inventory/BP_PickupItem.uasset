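; BP_PickupItem is an interactable world pickup that puts an item into the player's inventory.
; On BeginPlay it fills UIPickup from GetDefaultItemObject if unset; that function returns nothing here.
; On interaction it casts the interacting actor to BP_FPCharacter and tries adding UIPickup to its BPInventoryComponent.
; OnBlueprintValidatedInteract runs only when the add succeeds.
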(event `self.ReceiveBeginPlay`
  (if (not (`KismetSystemLibrary.IsValid` (`self.UIPickup`)))
    (bind _pickupitem (`self.GetDefaultItemObject`))
    (set `self.UIPickup` _pickupitem)))

(event `self.OnInteractEvent`
  (params (interactingCamera :type "SceneComponent Object Reference") (interactingActor :type "Actor Object Reference"))
  (if (and (`KismetSystemLibrary.IsValid` interactingCamera) (`KismetSystemLibrary.IsValid` interactingActor))
    (bind _asbp_fpcharacter (cast `/Game/BP_FPCharacter` interactingActor))
    (bind _success (`/Game/Inventory/SpatialInventory/BP_InventoryComponent2.TryAddItem` (`/Game/BP_FPCharacter.BP_InventoryComponent` _asbp_fpcharacter) (`self.UIPickup`)))
    (if _success
      (`self.OnBlueprintValidatedInteract` interactingCamera))))

(fn `GetDefaultItemObject`
  (returns (PickupItem :type "/Game/Inventory/BP_UIPickup Object Reference"))
  (return null))

(fn `UserConstructionScript`)
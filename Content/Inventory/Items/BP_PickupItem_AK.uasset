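; BP_PickupItem_AK is an AK-47 pickup item for the inventory system, derived from a parent pickup class.
; It overrides GetDefaultItemObject to construct and return a BP_UIPickup with the rifle's grid footprint, normal and rotated icons, and its own class as the pickup class.
; The event graph holds only disabled default events, and the construction script just calls the parent.
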(fn `GetDefaultItemObject`
  (returns (PickupItem :type "/Game/Inventory/BP_UIPickup Object Reference"))
  (bind _returnvalue (`|GenericCreateObject` self "/Game/Inventory/BP_UIPickup.BP_UIPickup_C" (make `IntPoint` 4 1) "/Game/FPS_Weapon_Bundle/Weapons/Icons/M_Icon_AK47.M_Icon_AK47" "/Game/FPS_Weapon_Bundle/Weapons/Icons/M_Icon_AK47_R.M_Icon_AK47_R" "BP_PickupItem_AK_C"))
  (return _returnvalue))

(fn `UserConstructionScript`
  (`parent.UserConstructionScript`))